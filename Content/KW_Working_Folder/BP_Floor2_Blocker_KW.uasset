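; Barrier actor that keeps the player from Floor 2 until enough Floor 1 puzzles are completed.
; Each Floor1PuzzleCompleted call increments a counter, and the blocker destroys itself when the counter reaches its maximum.
; Overlapping the box before then shows a "Scooby too scared" text widget for a few seconds, using a stored widget reference to avoid creating duplicates.
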(event OnComponentBeginOverlap(Box)
  (params (OverlappedComponent :type Primitive%20Component%20Object%20Reference) (OtherActor :type Actor%20Object%20Reference) (OtherComp :type Primitive%20Component%20Object%20Reference) (OtherBodyIndex :type Integer) (bFromSweep :type Boolean) (SweepResult :type Hit%20Result%20Structure%20%28by%20ref%29))
  (if (not (>= (Variables|Default|GetCurrentFloor1Puzzles) (Variables|Default|GetmaxFloor1Puzzles)))
    (Variables|Default|GetWidgetText
      (:then
        _)
      (:else
        ;[1 1 1] If Attic Incomplete, "Door Locked" Displays
        (bind _returnvalue (UserInterface|CreateWidget "/Game/KW_Working_Folder/BP_Text_ScoobyTooScared_KW.BP_Text_ScoobyTooScared_KW_C"))
        (Variables|Default|SetWidgetText _returnvalue)
        (UserInterface|Viewport|AddtoViewport _returnvalue 0)))
    (Utilities|FlowControl|Delay 3.0)
    (Widget|RemovefromParent _returnvalue)
    (Variables|Default|SetWidgetText 0)))

(event OnComponentHit(Box)
  (params (HitComponent :type Primitive%20Component%20Object%20Reference) (OtherActor :type Actor%20Object%20Reference) (OtherComp :type Primitive%20Component%20Object%20Reference) (NormalImpulse :type Vector :default "0, 0, 0") (Hit :type Hit%20Result%20Structure%20%28by%20ref%29)))

(event Custom|Floor1PuzzleCompleted
  (Math|Integer|IncrementInt (Variables|Default|GetCurrentFloor1Puzzles)
    (:%20%20
      (if (>= (Variables|Default|GetCurrentFloor1Puzzles) (Variables|Default|GetmaxFloor1Puzzles))
        (Utilities|FlowControl|DoOnce false
          (:Completed
            (Actor|DestroyActor)))))))

(event EventBeginPlay)

(event Collision|EventActorBeginOverlap
  (params (OtherActor :type Actor%20Object%20Reference)))

(event EventTick
  (params (DeltaSeconds :type Float%20%28single-precision%29)))

(fn ConstructionScript)