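; BP_F2R1_HintBox is a trigger actor that shows a hint when an actor overlaps it while the room is unlit.
; It reads RoomIsLit from BP_Clock, then CandleHeld from BP_Hold_Candlestick to pick either the "MoreLight" or "TooDark" text widget.
; A validity check on WidgetText prevents duplicate widgets, and a one-second delay precedes removing the widget and clearing the reference.
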(event Collision|EventActorBeginOverlap
  (params (OtherActor :type Actor%20Object%20Reference))
  ;[1 1 1] Hint Triggers Upon Player Overlap
  (bind _returnvalue (Actor|GetActorOfClass "/Game/Victorian_House/Blueprints/BP_Clock.BP_Clock_C"))
  (if (not (Variables|/Game/Victorian_House/Blueprints/BP_Clock.BP_Clock_C|GetRoomIsLit _returnvalue))
    (bind _returnvalue_2 (Actor|GetActorOfClass "/Game/KW_Working_Folder/BP_Hold_Candlestick.BP_Hold_Candlestick_C"))
    (if (Variables|/Game/KW_Working_Folder/BP_Hold_Candlestick.BP_Hold_Candlestick_C|GetCandleHeld _returnvalue_2)
      ;;[1 1 1] Hint if Candlestick in Hand
      (Variables|Default|GetWidgetText
        (:then
          _)
        (:else
          (bind _returnvalue_3 (UserInterface|CreateWidget "/Game/KW_Working_Folder/BP_Text_F2R1_MoreLight_KW.BP_Text_F2R1_MoreLight_KW_C"))
          (bind _output_get (Variables|Default|SetWidgetText _returnvalue_3))
          (UserInterface|Viewport|AddtoViewport _returnvalue_3 0)))
      (Utilities|FlowControl|Delay 1.0)
      (Widget|RemovefromParent _output_get)
      (Variables|Default|SetWidgetText 0)
      (else
        ;;[1 1 1] Hint if Candlestick is not Held
        (Variables|Default|GetWidgetText
          (:then
            _)
          (:else
            (bind _returnvalue_4 (UserInterface|CreateWidget "/Game/KW_Working_Folder/BP_Text_F2R1_TooDark_KW.BP_Text_F2R1_TooDark_KW_C"))
            (bind _output_get_2 (Variables|Default|SetWidgetText _returnvalue_4))
            (UserInterface|Viewport|AddtoViewport _returnvalue_4 0)))
        (Utilities|FlowControl|Delay 1.0)
        (Widget|RemovefromParent _output_get_2)
        (Variables|Default|SetWidgetText 0)))))

(fn ConstructionScript)