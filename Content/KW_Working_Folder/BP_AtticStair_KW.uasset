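; Attic stair actor that starts closed, shows a text widget on interact, and opens after the floor-3 puzzle completes or enough pages are collected.
; Page pickups increment a counter with timed popup widgets.
; Opening and closing play stair animations, briefly toggle the character's edit mode, and use paired DoOnce gates to alternate sounds and reposition ladder boxes.
; Box overlaps set the character's ladder state or toggle edit mode.
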(event OnComponentBeginOverlap(Box)
  (params (OverlappedComponent :type Primitive%20Component%20Object%20Reference) (OtherActor :type Actor%20Object%20Reference) (OtherComp :type Primitive%20Component%20Object%20Reference) (OtherBodyIndex :type Integer) (bFromSweep :type Boolean) (SweepResult :type Hit%20Result%20Structure%20%28by%20ref%29))
  ;[1 1 1] Attic_Ladder
  (bind _asbp_victorian_character (Utilities|Casting|CastToBP_VictorianCharacter OtherActor))
  (Variables|/Game/Victorian_House/Blueprints/BP_VictorianCharacter.BP_VictorianCharacter_C|SetIsOnLadder _asbp_victorian_character true))

(event OnComponentEndOverlap(Box)
  (params (OverlappedComponent :type Primitive%20Component%20Object%20Reference) (OtherActor :type Actor%20Object%20Reference) (OtherComp :type Primitive%20Component%20Object%20Reference) (OtherBodyIndex :type Integer))
  ;[1 1 1] Attic_Ladder
  (bind _asbp_victorian_character (Utilities|Casting|CastToBP_VictorianCharacter OtherActor))
  (Variables|/Game/Victorian_House/Blueprints/BP_VictorianCharacter.BP_VictorianCharacter_C|SetIsOnLadder _asbp_victorian_character false)
  (Pawn|Components|CharacterMovement|SetMovementMode (Variables|/Script/Engine.Character|GetCharacterMovement _asbp_victorian_character) "MOVE_Walking" 0))

(event OnComponentBeginOverlap(Box3)
  (params (OverlappedComponent :type Primitive%20Component%20Object%20Reference) (OtherActor :type Actor%20Object%20Reference) (OtherComp :type Primitive%20Component%20Object%20Reference) (OtherBodyIndex :type Integer) (bFromSweep :type Boolean) (SweepResult :type Hit%20Result%20Structure%20%28by%20ref%29))
  ;[1 1 1] Attic_Ladder
  (bind _asbp_victorian_character (Utilities|Casting|CastToBP_VictorianCharacter OtherActor))
  (Default|EditeModeOff _asbp_victorian_character))

(event OnComponentEndOverlap(Box3)
  (params (OverlappedComponent :type Primitive%20Component%20Object%20Reference) (OtherActor :type Actor%20Object%20Reference) (OtherComp :type Primitive%20Component%20Object%20Reference) (OtherBodyIndex :type Integer))
  ;[1 1 1] Attic_Ladder
  (bind _asbp_victorian_character (Utilities|Casting|CastToBP_VictorianCharacter OtherActor))
  (Default|EditeModeon _asbp_victorian_character))

(event Custom|CustomEvent
  (params (NewParam :type Boolean))
  ;[1 1 1] Outline
  (Utilities|FlowControl|DoN 1) ; enters at Reset
)

(event Custom|Collect_Items
  ;[1 1 1] Collects Items & Triggers Door Open
  (Math|Integer|IncrementInt (Variables|Default|GetcurrentItemsCollected)
    (:%20%20
      (bind _returnvalue (UserInterface|CreateWidget "/Game/KW_Working_Folder/BP_Text_PageCollectedCount_KW.BP_Text_PageCollectedCount_KW_C"))
      (UserInterface|Viewport|AddtoViewport _returnvalue 0)
      (Utilities|FlowControl|Delay 1.0)
      (Widget|RemovefromParent _returnvalue)
      (if (>= (Variables|Default|GetcurrentItemsCollected) (Variables|Default|GetmaxItemsCollected))
        (Utilities|FlowControl|DoOnce false
          (:Completed
            (Variables|Default|Setfloor2Complete true)
            (bind _returnvalue_2 (UserInterface|CreateWidget "/Game/KW_Working_Folder/BP_Text_PageCollectedLast_KW.BP_Text_PageCollectedLast_KW_C"))
            (UserInterface|Viewport|AddtoViewport _returnvalue_2 0)
            (Utilities|FlowControl|Delay 1.0)
            (Widget|RemovefromParent _returnvalue_2)
            (Viewport|RemoveAllWidgets)
            (CallFunction|OpenAttic)))))))

(event Custom|Completed_F3_Puzzle
  ;[1 1 1] Collects Items & Triggers Door Open
  (Variables|Default|SetcompletedAttic true)
  (Utilities|FlowControl|DoOnce false
    (:Completed
      (CallFunction|OpenAttic))))

(event Custom|Open_Attic
  (bind _box (Variables|Default|GetBox))
  (bind _box_2 (Variables|Default|GetBox))
  ;[1 1 1] Triggers Stairs to Open
  ;[1 1 1] Animation and Sound
  (Utilities|FlowControl|Sequence
    (:then_0
      (Utilities|FlowControl|DoOnce false
        (:Completed
          (Audio|PlaySoundatLocation "/Game/Victorian_House/Audio/Cues/Cue_CloseAtticStair.Cue_CloseAtticStair" "0, 0, 0" "0, 0, 0" 1.0 1.0 0.0 0 0 0 0)
          ;;[1 1 1] Begin Play -- Stairs Closed
          (Utilities|FlowControl|DoOnce false) ; enters at Reset
        )))
    (:then_1
      (Components|Animation|PlayAnimation (Variables|Default|GetSM_AtticStair) "/Game/Victorian_House/Animations/Anim_AtticStair_Open.Anim_AtticStair_Open" false)
      (Utilities|FlowControl|Sequence
        (:then_0
          (if true
            (bind _asbp_victorian_character (Utilities|Casting|CastToBP_VictorianCharacter (Game|GetPlayerCharacter 0)))
            (Default|EditeModeOff _asbp_victorian_character)
            (Utilities|FlowControl|Delay 2.0)
            (Default|EditeModeon _asbp_victorian_character)))
        (:then_1
          (Utilities|FlowControl|Delay 2.0)
          (Utilities|FlowControl|DoOnce false
            (:Completed
              (Transformation|AddRelativeRotation _box_2 "0, 0,-60.000000" false false)
              (Transformation|AddRelativeLocation _box_2 "0,0.000000,-160.000000" false false)
              (Utilities|FlowControl|DoOnce false) ; enters at Reset
            )))))))

(event Custom|Close_Attic
  (bind _box (Variables|Default|GetBox))
  (bind _box_2 (Variables|Default|GetBox))
  ;[1 1 1] Begin Play -- Stairs Closed
  ;[1 1 1] Animation and Sound
  (Variables|Default|SetinAttic true)
  (Utilities|FlowControl|Sequence
    (:then_0
      (if (Variables|Default|GetinAttic)
        (Utilities|FlowControl|DoOnce false
          (:Completed
            (Audio|PlaySoundatLocation "/Game/Victorian_House/Audio/Cues/Cue_OpenAtticStair.Cue_OpenAtticStair" "0, 0, 0" "0, 0, 0" 1.0 1.0 0.0 0 0 0 0)
            ;;[1 1 1] Triggers Stairs to Open
            (Utilities|FlowControl|DoOnce false) ; enters at Reset
          ))))
    (:then_1
      (Components|Animation|PlayAnimation (Variables|Default|GetSM_AtticStair) "/Game/Victorian_House/Animations/Anim_AtticStair_Close.Anim_AtticStair_Close" false)
      (Utilities|FlowControl|Sequence
        (:then_0
          (if true
            (bind _asbp_victorian_character (Utilities|Casting|CastToBP_VictorianCharacter (Game|GetPlayerCharacter 0)))
            (Default|EditeModeOff _asbp_victorian_character)
            (Utilities|FlowControl|Delay 2.0)
            (Default|EditeModeon _asbp_victorian_character)))
        (:then_1
          (Utilities|FlowControl|DoOnce false
            (:Completed
              (Transformation|AddRelativeRotation _box "0, 0,60.000000" false false)
              (Transformation|AddRelativeLocation _box "0,0.000000,160.000000" false false)
              (Utilities|FlowControl|DoOnce false) ; enters at Reset
            )))))))

(event EventOnFocus
  ;[1 1 1] Outline
)

(event EventOnInteract
  ;[1 1 1] Locked on Interact
  (Variables|Default|GetWidgetText
    (:then
      _)
    (:else
      (bind _returnvalue (UserInterface|CreateWidget "/Game/BH_Working_Folder/BP_Text_Attic_Stair.BP_Text_Attic_Stair_C"))
      (bind _output_get (Variables|Default|SetWidgetText _returnvalue))
      (UserInterface|Viewport|AddtoViewport _returnvalue 0)))
  (Utilities|FlowControl|Delay (Variables|Default|GetWidgetLength))
  (Widget|RemovefromParent _output_get)
  (Variables|Default|SetWidgetText 0))

(event EventBeginPlay
  (bind _box (Variables|Default|GetBox))
  (bind _box_2 (Variables|Default|GetBox))
  ;[1 1 1] Begin Play -- Stairs Closed
  ;[1 1 1] Animation and Sound
  (Utilities|FlowControl|Sequence
    (:then_0
      (if (Variables|Default|GetinAttic)
        (Utilities|FlowControl|DoOnce false
          (:Completed
            (Audio|PlaySoundatLocation "/Game/Victorian_House/Audio/Cues/Cue_OpenAtticStair.Cue_OpenAtticStair" "0, 0, 0" "0, 0, 0" 1.0 1.0 0.0 0 0 0 0)
            ;;[1 1 1] Triggers Stairs to Open
            (Utilities|FlowControl|DoOnce false) ; enters at Reset
          ))))
    (:then_1
      (Components|Animation|PlayAnimation (Variables|Default|GetSM_AtticStair) "/Game/Victorian_House/Animations/Anim_AtticStair_Close.Anim_AtticStair_Close" false)
      (Utilities|FlowControl|Sequence
        (:then_0
          (if true
            (bind _asbp_victorian_character (Utilities|Casting|CastToBP_VictorianCharacter (Game|GetPlayerCharacter 0)))
            (Default|EditeModeOff _asbp_victorian_character)
            (Utilities|FlowControl|Delay 2.0)
            (Default|EditeModeon _asbp_victorian_character)))
        (:then_1
          (Utilities|FlowControl|DoOnce false
            (:Completed
              (Transformation|AddRelativeRotation _box "0, 0,60.000000" false false)
              (Transformation|AddRelativeLocation _box "0,0.000000,160.000000" false false)
              (Utilities|FlowControl|DoOnce false) ; enters at Reset
            )))))))

(fn ConstructionScript)