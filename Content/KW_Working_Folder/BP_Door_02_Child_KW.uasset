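; Keycode-locked door that swings open on interaction once unlocked; the flip-flop's second branch is empty.
; While locked, interacting toggles a keypad widget and cursor, showing a timed hint chosen by BP_Clock's RoomIsLit.
; TryDoor compares the code, unlocking and restoring game input on a match.
; Focus shows an optional outline and a single prompt widget, cleared by a retriggerable delay.
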(event Custom|ResetWidget
  (params (NewParam :type Boolean))
  ;[1 1 1] Outline
  (Utilities|FlowControl|DoN 1) ; enters at Reset
)

(event Custom|Cancel
  (bind _returnvalue (Game|GetPlayerController 0))
  (Widget|RemovefromParent (stale EventOnInteract _output_get))
  (Variables|Default|SetPinWidgetRef 0)
  (Input|SetInputModeGameOnly _returnvalue false)
  (Variables|/Script/Engine.PlayerController|SetbShowMouseCursor _returnvalue false))

(event EventOnInteract
  (bind _returnvalue (Game|GetPlayerController 0))
  (bind _returnvalue_2 (Game|GetPlayerController 0))
  (if (Variables|Default|GetUnlocked)
    ;[1 1 1] Open Door
    (Utilities|FlowControl|FlipFlop
      (:A
        (Utilities|FlowControl|Sequence :!label _label
          (:then_0
            (Utilities|FlowControl|DoOnce false :!label _label_2
              (:Completed
                (Audio|PlaySoundatLocation "/Game/Victorian_House/Audio/Cues/Cue_OpenDoor_01.Cue_OpenDoor_01" "0, 0, 0" "0, 0, 0" 1.0 1.0 0.0 0 0 0 0)
                (Utilities|FlowControl|DoOnce false ; enters at Reset
                  (:Completed
                    (Audio|PlaySoundatLocation "/Game/Victorian_House/Audio/Cues/Cue_CloseDoor_01.Cue_CloseDoor_01" "0, 0, 0" "0, 0, 0" 1.0 1.0 0.0 0 0 0 0)
                    (goto _label_2 Reset))))))
          (:then_1
            (bind _doorrotater (Timeline|Timeline Play)
              (:Update
                (Transformation|SetRelativeRotation (Variables|Default|GetMesh_Door_02) (Math|Rotator|MakeRotator 0.0 0.0 _doorrotater) false false))))))
      (:B
        (Utilities|FlowControl|Sequence)))
    (else
      (Utilities|IsValid (Variables|Default|GetPinWidgetRef)
        (:Is%20Valid
          (Widget|RemovefromParent (stale _output_get))
          (Variables|Default|SetPinWidgetRef 0)
          (Input|SetInputModeGameOnly _returnvalue_2 false)
          (Variables|/Script/Engine.PlayerController|SetbShowMouseCursor _returnvalue_2 false))
        (:Is%20Not%20Valid
          (bind _returnvalue_3 (UserInterface|CreateWidget "/Game/KW_Working_Folder/BP_Widget_KeyCode_KW.BP_Widget_KeyCode_KW_C" 0 self))
          (bind _output_get (Variables|Default|SetPinWidgetRef _returnvalue_3))
          (UserInterface|Viewport|AddtoViewport _output_get 0)
          (Input|SetInputModeGameandUI _returnvalue 0 "DoNotLock" false false)
          (Variables|/Script/Engine.PlayerController|SetbShowMouseCursor _returnvalue true)
          (if (Variables|Default|GetUnlocked)
            (goto _label)
            (else
              (bind _returnvalue_4 (Actor|GetActorOfClass "/Game/Victorian_House/Blueprints/BP_Clock.BP_Clock_C"))
              (if (Variables|/Game/Victorian_House/Blueprints/BP_Clock.BP_Clock_C|GetRoomIsLit _returnvalue_4)
                (Variables|Default|GetWidgetText
                  (:then
                    _)
                  (:else
                    (bind _returnvalue_5 (UserInterface|CreateWidget "/Game/KW_Working_Folder/BP_Text_F2R2_TimeHint_KW.BP_Text_F2R2_TimeHint_KW_C"))
                    (bind _output_get_2 (Variables|Default|SetWidgetText _returnvalue_5))
                    (UserInterface|Viewport|AddtoViewport _returnvalue_5 0)))
                (Utilities|FlowControl|Delay 5.0)
                (Widget|RemovefromParent _output_get_2)
                (Variables|Default|SetWidgetText 0)
                (else
                  (Variables|Default|GetWidgetText
                    (:then
                      _)
                    (:else
                      (bind _returnvalue_6 (UserInterface|CreateWidget "/Game/KW_Working_Folder/BP_Text_F2R2_EarlyHint_KW.BP_Text_F2R2_EarlyHint_KW_C"))
                      (bind _output_get_3 (Variables|Default|SetWidgetText _returnvalue_6))
                      (UserInterface|Viewport|AddtoViewport _returnvalue_6 0)))
                  (Utilities|FlowControl|Delay 3.0)
                  (Widget|RemovefromParent _output_get_3)
                  (Variables|Default|SetWidgetText 0))))))))))

(event Collision|EventActorBeginOverlap
  (params (OtherActor :type Actor%20Object%20Reference))
  ;[1 1 1] Open Door
  (Utilities|FlowControl|Sequence))

(event EventOnFocus
  ;[1 1 1] Outline
  (Utilities|FlowControl|Sequence
    (:then_0
      (if (Variables|Default|GetOutline%20on/off)
        (CallFunction|BeginFocus))
      (Variables|Default|SetTimeOutlineEnd 0.1)
      (Utilities|FlowControl|RetriggerableDelay (Variables|Default|GetTimeOutlineEnd))
      (CallFunction|EndFocus)
      (Widget|RemovefromParent (stale _returnvalue))
      (CallFunction|ResetWidget false))
    (:then_1
      (Utilities|FlowControl|DoN 1
        (:Exit
          (bind _returnvalue (UserInterface|CreateWidget "/Game/Victorian_House/UMG/Door_Widget.Door_Widget_C"))
          (UserInterface|Viewport|AddtoViewport _returnvalue 0))))))

(fn ConstructionScript
  (|CallParentFunction))

(fn TryDoor
  (params (Door%20Code :type String))
  (bind _returnvalue (Game|GetPlayerController 0))
  (if (Utilities|Enum|Equal(Enum) Door%20Code (Variables|Default|GetKeyCode))
    (Variables|Default|SetUnlocked true)
    (Widget|RemovefromParent (Variables|Default|GetPinWidgetRef))
    (Input|SetInputModeGameOnly _returnvalue false)
    (Variables|/Script/Engine.PlayerController|SetbShowMouseCursor _returnvalue false)
    (return (Variables|Default|GetUnlocked))))