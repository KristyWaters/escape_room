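; A three-flame candlestick that lights up when the Victorian player character comes near while carrying the held candle.
; On BeginPlay it hides its three flame particles and three point lights.
; Overlapping LightProximity checks CandleHeld on BP_Hold_Candlestick, found by class, then reveals the flames and lights and calls LightCandlesticks on that actor.
; Some leftover disconnected nodes never run.
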(event OnComponentBeginOverlap(LightProximity)
  (params (OverlappedComponent :type Primitive%20Component%20Object%20Reference) (OtherActor :type Actor%20Object%20Reference) (OtherComp :type Primitive%20Component%20Object%20Reference) (OtherBodyIndex :type Integer) (bFromSweep :type Boolean) (SweepResult :type Hit%20Result%20Structure%20%28by%20ref%29))
  (Utilities|Casting|CastToBP_VictorianCharacter OtherActor)
  (bind _returnvalue (Actor|GetActorOfClass "/Game/KW_Working_Folder/BP_Hold_Candlestick.BP_Hold_Candlestick_C"))
  (if (Variables|/Game/KW_Working_Folder/BP_Hold_Candlestick.BP_Hold_Candlestick_C|GetCandleHeld _returnvalue)
    (Development|SetHiddeninGame (Variables|Default|GetP_Candle_Fire) false false)
    (Development|SetHiddeninGame (Variables|Default|GetP_Candle_Fire1) false false)
    (Development|SetHiddeninGame (Variables|Default|GetP_Candle_Fire2) false false)
    (Development|SetHiddeninGame (Variables|Default|GetPointLight) false false)
    (Development|SetHiddeninGame (Variables|Default|GetPointLight1) false false)
    (Development|SetHiddeninGame (Variables|Default|GetPointLight2) false false)
    (bind _returnvalue_2 (Actor|GetActorOfClass "/Game/KW_Working_Folder/BP_Hold_Candlestick.BP_Hold_Candlestick_C"))
    (Default|LightCandlesticks _returnvalue_2)))

(event EventBeginPlay
  (Development|SetHiddeninGame (Variables|Default|GetP_Candle_Fire) true false)
  (Development|SetHiddeninGame (Variables|Default|GetP_Candle_Fire1) true false)
  (Development|SetHiddeninGame (Variables|Default|GetP_Candle_Fire2) true false)
  (Development|SetHiddeninGame (Variables|Default|GetPointLight) true false)
  (Development|SetHiddeninGame (Variables|Default|GetPointLight1) true false)
  (Development|SetHiddeninGame (Variables|Default|GetPointLight2) true false))

(fn ConstructionScript)