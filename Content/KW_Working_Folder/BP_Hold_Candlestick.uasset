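; Candlestick interactable that tracks whether the Victorian character is holding an item and counts lit candles to light the room.
; Focus shows an optional outline and a Look widget, both cleared by a retriggerable delay once focus calls stop, while interacting toggles the widget.
; Each LightCandlesticks call increments the count; at the maximum, it switches on every BP_F2R1_Light once and sets RoomIsLit on BP_Clock.
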(event Custom|LightCandlesticks
  ;[1 1 1] Light Candlesticks Function
  (Math|Integer|IncrementInt (Variables|Default|GetLitCandles)
    (:%20%20
      (if (>= (Variables|Default|GetLitCandles) (Variables|Default|GetMaxCandles))
        (Utilities|FlowControl|DoOnce false
          (:Completed
            (bind _outactors (Actor|GetAllActorsOfClass "/Game/KW_Working_Folder/BP_F2R1_Light.BP_F2R1_Light_C"))
            (for _array_element _outactors
              (Default|CenterLighton _array_element))
            (bind _returnvalue (Actor|GetActorOfClass "/Game/Victorian_House/Blueprints/BP_Clock.BP_Clock_C"))
            (Variables|/Game/Victorian_House/Blueprints/BP_Clock.BP_Clock_C|SetRoomIsLit _returnvalue true)))))))

(event Custom|Reset2
  (params (NewParam :type Boolean))
  ;[1 1 1] Outline
  (Utilities|FlowControl|DoN 1) ; enters at Reset
)

(event EventOnFocus
  ;[1 1 1] Outline
  (bind _returnvalue (Actor|GetActorOfClass "/Game/Victorian_House/Blueprints/BP_VictorianCharacter.BP_VictorianCharacter_C"))
  (if (Variables|/Game/Victorian_House/Blueprints/BP_VictorianCharacter.BP_VictorianCharacter_C|GetIsHolding _returnvalue)
    (Variables|Default|SetCandleHeld true)
    (else
      (Variables|Default|SetCandleHeld false)))
  (Utilities|FlowControl|Sequence
    (:then_0
      (if (Variables|Default|GetOutline%20on/off)
        (CallFunction|BeginFocus))
      (Variables|Default|SetTimeOutlineEnd 0.1)
      (Utilities|FlowControl|RetriggerableDelay (Variables|Default|GetTimeOutlineEnd))
      (CallFunction|EndFocus)
      (Widget|RemovefromParent (stale _returnvalue_2))
      (CallFunction|Reset2 false))
    (:then_1
      (Utilities|FlowControl|DoN 1
        (:Exit
          (bind _returnvalue_2 (UserInterface|CreateWidget "/Game/Victorian_House/UMG/Look_Widget.Look_Widget_C")) ; Change widget for Edit Mode
          (UserInterface|Viewport|AddtoViewport _returnvalue_2 0))))))

(event EventOnInteract
  ;[1 1 1] Widget on/off
  (bind _returnvalue (Actor|GetActorOfClass "/Game/Victorian_House/Blueprints/BP_VictorianCharacter.BP_VictorianCharacter_C"))
  (if (Variables|/Game/Victorian_House/Blueprints/BP_VictorianCharacter.BP_VictorianCharacter_C|GetIsHolding _returnvalue)
    (Variables|Default|SetCandleHeld true)
    (else
      (Variables|Default|SetCandleHeld false)))
  (Utilities|FlowControl|FlipFlop
    (:A
      (Widget|RemovefromParent (stale EventOnFocus _returnvalue_2)))
    (:B
      (UserInterface|Viewport|AddtoViewport (stale EventOnFocus _returnvalue_2) 0))))

(fn ConstructionScript
  (|CallParentFunction))