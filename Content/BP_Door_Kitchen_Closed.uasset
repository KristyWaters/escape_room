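; Kitchen door Blueprint holding logic to swing MeshDoor02 open and closed and show a focus prompt, all currently disconnected.
; A FlipFlop plays or reverses a yaw Timeline, with DoOnce nodes gating open and close sounds at world origin.
; The focus chain uses a retriggerable delay to clear the outline and Door_Widget, with DoN limiting widget creation.
; OnInteract and OnFocus are empty, so neither chain runs.
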(event Custom|CustomEvent
  (params (NewParam :type Boolean))
  ;[1 1 1] Outline
  (Utilities|FlowControl|DoN 1) ; enters at Reset
)

(event EventOnInteract
  ;[1 1 1] Open Door
)

(event Collision|EventActorBeginOverlap
  (params (OtherActor :type Actor%20Object%20Reference))
  ;[1 1 1] Open Door
)

(event EventOnFocus
  ;[1 1 1] Outline
)

(fn ConstructionScript)