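; Chess board actor for a puzzle that detects whether its assigned chess piece is placed on it.
; When a chess piece enters the ChessBox trigger, it is compared to ChessMatch; a match sets CorrectPiece and calls CallCheckDrawers.
; Removing the matching piece clears the flag without calling CallCheckDrawers again.
; Feedback for right and wrong pieces is debug text, with text widgets still marked TODO.
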(event OnComponentBeginOverlap(ChessBox)
  (params (OverlappedComponent :type Primitive%20Component%20Object%20Reference) (OtherActor :type Actor%20Object%20Reference) (OtherComp :type Primitive%20Component%20Object%20Reference) (OtherBodyIndex :type Integer) (bFromSweep :type Boolean) (SweepResult :type Hit%20Result%20Structure%20%28by%20ref%29))
  ;[1 1 1] Check for correct Chess Piece -> TODO: Add text widgets
  (bind _asbp_chess_piece (Utilities|Casting|CastToBP_ChessPiece OtherActor))
  (if (== _asbp_chess_piece (Variables|Default|GetChessMatch))
    (Development|PrintString "You did it!")
    (Variables|Default|SetCorrectPiece true)
    (Default|CallCheckDrawers)
    (else
      (Development|PrintString "Wront Piece"))))

(event OnComponentEndOverlap(ChessBox)
  (params (OverlappedComponent :type Primitive%20Component%20Object%20Reference) (OtherActor :type Actor%20Object%20Reference) (OtherComp :type Primitive%20Component%20Object%20Reference) (OtherBodyIndex :type Integer))
  ;[1 1 1] Reverse if removed
  (bind _asbp_chess_piece (Utilities|Casting|CastToBP_ChessPiece OtherActor))
  (if (== _asbp_chess_piece (Variables|Default|GetChessMatch))
    (Variables|Default|SetCorrectPiece false)))

(event EventBeginPlay)

(event Collision|EventActorBeginOverlap
  (params (OtherActor :type Actor%20Object%20Reference)))

(event EventTick
  (params (DeltaSeconds :type Float%20%28single-precision%29)))

(fn ConstructionScript)