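; BP_Light_Button is the submit button for a light color puzzle that unlocks a door.
; On interact it compares each puzzle piece's color index with the matching ColorCode entry, stopping at the first mismatch.
; A full match calls UnlockDoor, while any mismatch resets every piece to color index zero and refreshes its light.
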(event EventBeginPlay)

(event Collision|EventActorBeginOverlap
  (params (OtherActor :type Actor%20Object%20Reference)))

(event EventTick
  (params (DeltaSeconds :type Float%20%28single-precision%29)))

(event EventOnInteract
  (Variables|Default|SetCorrect true)
  (bind (_array_element _array_index) (Utilities|Array|ForEachLoopwithBreak (Variables|Default|GetPuzzlePieces) :!label _label)
    (:LoopBody
      (if (!= (Variables|/Game/BH_Working_Folder/LightPuzzle/BP_Light_PuzzlePiece.BP_Light_PuzzlePiece_C|GetColorIndex _array_element) (Utilities|Array|Get(acopy) (Variables|Default|GetColorCode) _array_index))
        (Variables|Default|SetCorrect false)
        (goto _label Break)))
    (:Completed
      (if (Variables|Default|GetCorrect)
        (Default|CallUnlockDoor)
        (else
          (for _array_element_2 (Variables|Default|GetPuzzlePieces)
            (Variables|/Game/BH_Working_Folder/LightPuzzle/BP_Light_PuzzlePiece.BP_Light_PuzzlePiece_C|SetColorIndex _array_element_2 0)
            (Default|UpdateLightColor _array_element_2)))))))

(fn ConstructionScript)