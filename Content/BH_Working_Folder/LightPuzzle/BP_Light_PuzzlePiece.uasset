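; Light puzzle piece whose point light cycles through four preset colors as it is interacted with.
; OnInteract increments ColorIndex, wraps it back to zero after the last color, then calls UpdateLightColor to apply the matching color.
; OnFocus is empty, and the piece itself holds no solution check.
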(event EventBeginPlay)

(event Collision|EventActorBeginOverlap
  (params (OtherActor :type Actor%20Object%20Reference)))

(event EventTick
  (params (DeltaSeconds :type Float%20%28single-precision%29)))

(event EventOnFocus)

(event EventOnInteract
  (bind _result (Math|Integer|IncrementInt (Variables|Default|GetColorIndex))
    (:%20%20
      (if (<= _result 3)
        _
        (else
          (Variables|Default|SetColorIndex 0)))
      (CallFunction|UpdateLightColor))))

(fn ConstructionScript)

(fn UpdateLightColor
  (bind _pointlight (Variables|Default|GetPointLight))
  (switch int (Variables|Default|GetColorIndex)
    (:0
      (Rendering|Components|Light|SetLightColor _pointlight "(R=1.000000,G=1.000000,B=1.000000,A=1.000000)" true))
    (:1
      (Rendering|Components|Light|SetLightColor _pointlight "(R=1.000000,G=0.262106,B=0.773299,A=1.000000)" true))
    (:2
      (Rendering|Components|Light|SetLightColor _pointlight "(R=0.192456,G=0.593492,B=1.000000,A=1.000000)" true))
    (:3
      (Rendering|Components|Light|SetLightColor _pointlight "(R=0.156314,G=1.000000,B=0.197167,A=1.000000)" true))))