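; BP_Light_Puzzle_Lamp is an interactable lamp for the light puzzle that stays locked until the chess puzzle is completed.
; On BeginPlay it binds to ChessDrawer's LightsActivateable event, which makes it interactable, turns on its PointLight and plays a sound.
; Each interaction then cycles the light through four colors via UpdateLightColor; while locked, it only prints a refusal message.
; The construction script sets the light's initial visibility from LightOnoff.
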(event Custom|LightsOn
  ;[1 1 1] Activate Light Puzzle when Chess Puzzle complete
  (Variables|Default|SetInteractable true)
  (Variables|Default|SetLight%20on/off%20 true)
  (Rendering|SetVisibility (Variables|Default|GetPointLight) (Variables|Default|GetLight%20on/off%20) false)
  (Audio|PlaySoundatLocation "/Game/Victorian_House/Audio/Cues/Cue_Light.Cue_Light" "0, 0, 0" "0, 0, 0" 1.0 1.0 0.0 0 0 0 0))

(event EventBeginPlay
  ;[1 1 1] Activate Light Puzzle when Chess Puzzle complete
  (EventDispatchers|BindEventtoLightsActivateable (Variables|Default|GetChessDrawer) (delegate Custom|LightsOn)))

(event EventOnInteract
  ;[1 1 1] Click to change color
  (if (Variables|Default|GetInteractable)
    (bind _result (Math|Integer|IncrementInt (Variables|Default|GetColorIndex))
      (:%20%20
        (if (<= _result 3)
          _
          (else
            (Variables|Default|SetColorIndex 0)))
        (CallFunction|UpdateLightColor)
        (Audio|PlaySoundatLocation "/Game/Victorian_House/Audio/Cues/Cue_Light.Cue_Light" "0, 0, 0" "0, 0, 0" 1.0 1.0 0.0 0 0 0 0)))
    (else
      (Development|PrintString "Some force prevents you from turning this on"))))

(fn ConstructionScript
  ;[1 1 1] on/off Light
  (Rendering|SetVisibility (Variables|Default|GetPointLight) (Variables|Default|GetLight%20on/off%20) false))

(fn UpdateLightColor
  (bind _pointlight (Variables|Default|GetPointLight))
  ;[1 1 1] Set Color to one of four options
  (switch int (Variables|Default|GetColorIndex)
    (:0
      (Rendering|Components|Light|SetLightColor _pointlight "(R=1.000000,G=1.000000,B=1.000000,A=1.000000)" true))
    (:1
      (Rendering|Components|Light|SetLightColor _pointlight "(R=1.000000,G=0.322356,B=0.830589,A=1.000000)" true))
    (:2
      (Rendering|Components|Light|SetLightColor _pointlight "(R=0.380405,G=0.721226,B=1.000000,A=1.000000)" true))
    (:3
      (Rendering|Components|Light|SetLightColor _pointlight "(R=0.407633,G=1.000000,B=0.281779,A=1.000000)" true))))