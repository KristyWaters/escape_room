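; BP_Gate is a puzzle gate that raises and drops in response to a linked pedestal object.
; On BeginPlay it caches the gate's start location, binds the pedestal's Pedestal and NoPedestal dispatchers to RaiseGate and DropGate, and drops unless flagged Open.
; One timeline lerps the gate toward EndLocation when dropping and reverses to raise it, with a sound for each direction.
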(event Custom|DropGate
  ;[1 1 1] Raise and Lower Gate
  (Audio|PlaySoundatLocation "/Engine/VREditor/Sounds/UI/Dockable_Window_Drop.Dockable_Window_Drop" (Transformation|GetWorldLocation (Variables|Default|GetGate)) "0, 0, 0" 0.5 1.0 0.0 0 0 0 0)
  (bind _alpha (Timeline|GateMovement Play)
    (:Update
      (Transformation|SetRelativeLocation (Variables|Default|GetGate) (Math|Vector|Lerp(Vector) (Variables|Default|GetStartingLocation) (Variables|Default|GetEndLocation) _alpha) false false))))

(event Custom|RaiseGate
  ;[1 1 1] Raise and Lower Gate
  (Audio|PlaySoundatLocation "/Engine/VREditor/Sounds/UI/Dockable_Window_Open.Dockable_Window_Open" (Transformation|GetWorldLocation (Variables|Default|GetGate)) "0, 0, 0" 0.5 1.0 0.0 0 0 0 0)
  (bind _alpha (Timeline|GateMovement Reverse)
    (:Update
      (Transformation|SetRelativeLocation (Variables|Default|GetGate) (Math|Vector|Lerp(Vector) (Variables|Default|GetStartingLocation) (Variables|Default|GetEndLocation) _alpha) false false))))

(event EventBeginPlay
  (bind _pedestalobject (Variables|Default|GetPedestalObject))
  (Variables|Default|SetStartingLocation (Variables|/Script/Engine.SceneComponent|GetRelativeLocation (Variables|Default|GetGate)))
  ;[1 1 1] Bind to Event Dispatcher
  (EventDispatchers|BindEventtoNoPedestal _pedestalobject (delegate Custom|DropGate))
  (EventDispatchers|BindEventtoPedestal _pedestalobject (delegate Custom|RaiseGate))
  ;[1 1 1] TODO -> Remove sound for this instance
  (if (not (Variables|Default|GetOpen))
    (CallFunction|DropGate)))

(fn ConstructionScript)