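; BP_Gate is a gate that raises and lowers in response to a linked pedestal object.
; On BeginPlay it stores the gate's starting relative location and binds to the pedestal's dispatchers, with NoPedestal raising the gate and Pedestal lowering it.
; Raising plays the GateMovement timeline, which lerps the gate from its start to EndLocation, and lowering reverses that same timeline.
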(event Custom|RaiseGate
  ;[1 1 1] Raise and Lower Gate
  (bind _alpha (Timeline|GateMovement Play)
    (:Update
      (Transformation|SetRelativeLocation (Variables|Default|GetGate) (Math|Vector|Lerp(Vector) (Variables|Default|GetStartingLocation) (Variables|Default|GetEndLocation) _alpha) false false))))

(event Custom|LowerGate
  ;[1 1 1] Raise and Lower Gate
  (bind _alpha (Timeline|GateMovement Reverse)
    (:Update
      (Transformation|SetRelativeLocation (Variables|Default|GetGate) (Math|Vector|Lerp(Vector) (Variables|Default|GetStartingLocation) (Variables|Default|GetEndLocation) _alpha) false false))))

(event EventBeginPlay
  (bind _pedestalobject (Variables|Default|GetPedestalObject))
  (Variables|Default|SetStartingLocation (Variables|/Script/Engine.SceneComponent|GetRelativeLocation (Variables|Default|GetGate)))
  ;[1 1 1] Bind to Event Dispatcher
  (EventDispatchers|BindEventtoNoPedestal _pedestalobject (delegate Custom|RaiseGate))
  (EventDispatchers|BindEventtoPedestal _pedestalobject (delegate Custom|LowerGate)))

(event Collision|EventActorBeginOverlap
  (params (OtherActor :type Actor%20Object%20Reference)))

(event EventTick
  (params (DeltaSeconds :type Float%20%28single-precision%29)))

(fn ConstructionScript)